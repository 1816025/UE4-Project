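; Key actor Blueprint with a static mesh and a replicated flag that removes the key from the game.
; On BeginPlay, a second actor tag of "1" swaps the mesh material to BasicAsset01.
; The flag's OnRep handler destroys the actor; nothing in this Blueprint sets the flag.
; An unconnected leftover graph would cycle a color parameter every five seconds, but its parameter name is None.
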(event EventBeginPlay
  (if (Utilities|Name|Equal(Name) (Utilities|Array|Get(acopy) (Variables|Actor|GetTags) 1) "1")
    (Rendering|Material|SetMaterial (Variables|Debug|GetStaticMeshComponent) 0 "/Engine/MapTemplates/Materials/BasicAsset01.BasicAsset01")))

(fn ConstructionScript)

(fn OnRepFlag
  (Actor|DestroyActor))