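; BP_MakeItem is a map item spawner that replaces three placeholder cube components with random rune actors on BeginPlay.
; RandomItem processes each cube in sequence, spawning a scaled-down Kano, Box Kano, Ing or Isa rune at its location, then destroying it.
; An empty fifth Select option leaves some spots without a rune.
; The RandomInteger(5) == 5 skip check never passes, and its branches all lead to destroying the first cube.
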(event EventBeginPlay
  (CallFunction|RandomItem (Variables|Default|GetCube1) (Variables|Default|GetCube2) (Variables|Default|GetCube3)))

(event Collision|EventActorBeginOverlap
  (params (OtherActor :type Actor%20Object%20Reference)))

(event EventTick
  (params (DeltaSeconds :type Float%20%28single-precision%29)))

(fn ConstructionScript)

(fn RandomItem
  (params (ターゲット :type Scene%20Component%20Object%20Reference) (ターゲット1 :type Scene%20Component%20Object%20Reference) (ターゲット2 :type Scene%20Component%20Object%20Reference))
  (bind _returnvalue (Math|Random|RandomInteger 5))
  (bind _returnvalue_2 (== _returnvalue 5))
  (bind _returnvalue_3 (Utilities|Select :Index _returnvalue :Option%200 "/Game/item/BP/Rune_Kano.Rune_Kano_C" :Option%201 "/Game/item/BP/Rune_Box_Kano.Rune_Box_Kano_C" :Option%202 "/Game/item/BP/Rune_ing.Rune_ing_C" :Option%203 "/Game/item/BP/Rune_Isa.Rune_Isa_C" :Option%204 0))
  (Utilities|FlowControl|Sequence
    (:then_0
      (if _returnvalue_2
        _
        (else
          (Game|SpawnActorfromClass _returnvalue_3 (Math|Transform|MakeTransform (Transformation|GetWorldLocation ターゲット) "0, 0, 0" "0.750000,0.750000,0.750000") "Undefined" 0 0)))
      (Components|DestroyComponent ターゲット :!label _label))
    (:then_1
      (if _returnvalue_2
        (goto _label)
        (else
          (Game|SpawnActorfromClass _returnvalue_3 (Math|Transform|MakeTransform (Transformation|GetWorldLocation ターゲット1) "0, 0, 0" "0.750000,0.750000,0.750000") "Undefined" 0 0)
          (Components|DestroyComponent ターゲット1))))
    (:then_2
      (if _returnvalue_2
        (goto _label)
        (else
          (Game|SpawnActorfromClass _returnvalue_3 (Math|Transform|MakeTransform (Transformation|GetWorldLocation ターゲット2) "0, 0, 0" "0.750000,0.750000,0.750000") "Undefined" 0 0)
          (Components|DestroyComponent ターゲット2))))))