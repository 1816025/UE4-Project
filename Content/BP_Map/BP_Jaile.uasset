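; BP_Jaile is a map actor, apparently a jail, that populates itself with BP_MakeItem actors when play begins.
; BeginPlay calls MakeDesk, which loops over a fixed set of placeholder Cube components.
; Each cube marks a spawn point: a BP_MakeItem spawns at its world location, then the cube is destroyed.
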(event EventBeginPlay
  (CallFunction|MakeDesk))

(event Collision|EventActorBeginOverlap
  (params (OtherActor :type Actor%20Object%20Reference)))

(event EventTick
  (params (DeltaSeconds :type Float%20%28single-precision%29)))

(fn ConstructionScript)

(fn MakeDesk
  (for _array_element (Utilities|Array|MakeArray (Variables|Default|GetCube) (Variables|Default|GetCube1) (Variables|Default|GetCube2) (Variables|Default|GetCube3) (Variables|Default|GetCube4) (Variables|Default|GetCube7) (Variables|Default|GetCube8) (Variables|Default|GetCube9) (Variables|Default|GetCube11) (Variables|Default|GetCube12))
    (Game|SpawnActorfromClass "/Game/BP_Map/BP_MakeItem.BP_MakeItem_C" (Math|Transform|MakeTransform (Transformation|GetWorldLocation _array_element) "0, 0, 0" "1,1,1") "Undefined" 0 0)
    (Components|DestroyComponent _array_element)))