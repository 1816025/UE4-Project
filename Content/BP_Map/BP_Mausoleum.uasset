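; Mausoleum puzzle actor that opens a hidden passage once five statue stands are completed.
; GoalGimmick takes a stand name, and on its first completion decrements player 0's StoneBoard count, spawns a Key_BP above that stand and flags it in a map.
; When all five flags are true, it spawns MoveDoor1 at Cube5 and destroys the crypt wall decoration and gargoyle, switching on authority between a direct event and a RunOfServer variant.
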(event Custom|SpawnMoveDoor1_RunOfServer
  (params (X :type Float%20%28single-precision%29) (Y :type Float%20%28single-precision%29) (Z :type Float%20%28single-precision%29))
  (Game|SpawnActorfromClass "/Game/MoveDoor1.MoveDoor1_C" (Math|Transform|MakeTransform (Math|Vector|MakeVector X Y Z) "0, 0, 0" "1,1,1") "Undefined" 0 0)
  (Components|DestroyComponent (Variables|Default|GetSM_Crypt_Wall_Decorative_D)))

(event Custom|spawnMoveDoor1
  (params (X :type Float%20%28single-precision%29) (Y :type Float%20%28single-precision%29) (Z :type Float%20%28single-precision%29))
  (Game|SpawnActorfromClass "/Game/MoveDoor1.MoveDoor1_C" (Math|Transform|MakeTransform (Math|Vector|MakeVector X Y Z) "0, 0, 0" "1,1,1") "Undefined" 0 0)
  (Components|DestroyComponent (Variables|Default|GetSM_Crypt_Wall_Decorative_D)))

(event EventBeginPlay
  (Variables|Default|SetNewVar_1 (Utilities|Map|MakeMap "SM_Statue_Stand" (Variables|Default|GetSM_Statue_Stand) "SM_Statue_Stand1" (Variables|Default|GetSM_Statue_Stand1) "SM_Statue_Stand2" (Variables|Default|GetSM_Statue_Stand2) "SM_Statue_Stand3" (Variables|Default|GetSM_Statue_Stand3) "SM_Statue_Stand4" (Variables|Default|GetSM_Statue_Stand4)))
  (Variables|Default|SetNewVar_3 (.AsFirst%20Person%20Character (Utilities|Casting|CastToFirstPersonCharacter (Game|GetPlayerCharacter 0)))))

(event Collision|EventActorBeginOverlap
  (params (OtherActor :type Actor%20Object%20Reference)))

(event EventTick
  (params (DeltaSeconds :type Float%20%28single-precision%29)))

(event EventGoalGimmick
  (params (NewParam :type Name :default "None"))
  (bind _newvar_3 (Variables|Default|GetNewVar_3))
  (bind _newvar_0 (Variables|Default|GetNewVar_0))
  (bind _cube5 (Variables|Default|GetCube5))
  (bind _newvar_1 (Variables|Default|GetNewVar_1))
  (bind _newvar_0_2 (Variables|Default|GetNewVar_0))
  (bind _returnvalue (Transformation|GetWorldLocation _cube5))
  (bind _value (Utilities|Map|Find _newvar_1 NewParam))
  (bind (_value_2 _returnvalue_2) (Utilities|Map|Find _newvar_0_2 NewParam))
  (bind _returnvalue_3 (Transformation|GetWorldLocation _value))
  (Utilities|FlowControl|Sequence
    (:then_0
      (if _returnvalue_2
        (if (not _value_2)
          (Variables|/Game/FirstPersonBP/Blueprints/FirstPersonCharacter.FirstPersonCharacter_C|SetStone%20board _newvar_3 (- (Variables|/Game/FirstPersonBP/Blueprints/FirstPersonCharacter.FirstPersonCharacter_C|GetStone%20board _newvar_3) 1))
          (Game|SpawnActorfromClass "/Game/key_BP.key_BP_C" (Math|Transform|MakeTransform (Math|Vector|MakeVector (.x _returnvalue_3) (.y _returnvalue_3) (+ (.z _returnvalue_3) 55.0)) "0, 0, 0" "1,1,1") "Undefined" 0 0)
          (bind _output_get (Variables|Default|SetNewVar_2 true))
          (Utilities|Map|Add _newvar_0 NewParam _output_get)
          (bind _values (Utilities|Map|Values _newvar_0)))))
    (:then_1
      (bind (_array_element _array_index) (Utilities|Array|ForEachLoopwithBreak _values :!label _label)
        (:LoopBody
          (if _array_element
            (if (== _array_index 4)
              (Networking|SwitchHasAuthority
                (:Authority
                  (CallFunction|SpawnMoveDoor1 (.x _returnvalue) (.y _returnvalue) (.z _returnvalue)))
                (:Remote
                  (CallFunction|SpawnMoveDoor1RunOfServer (.x _returnvalue) (.y _returnvalue) (.z _returnvalue)))))
            (else
              (goto _label Break))))))))

(fn ConstructionScript)