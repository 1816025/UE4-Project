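; Wall map piece that randomly places rune pickups at its eight cube components when play begins.
; For each cube, RandomItem makes a chance roll, then a second roll selects one of four rune classes or an empty slot.
; A chosen rune spawns scaled down at the cube's world location.
; Every cube is destroyed afterwards whether or not anything spawns, so the cubes act only as placement markers.
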(event EventBeginPlay
  (Utilities|FlowControl|Sequence
    (:then_0
      (CallFunction|RandomItem (Variables|Default|GetCube1)))
    (:then_1
      (CallFunction|RandomItem (Variables|Default|GetCube2)))
    (:then_2
      (CallFunction|RandomItem (Variables|Default|GetCube5)))
    (:then_3
      (CallFunction|RandomItem (Variables|Default|GetCube6)))
    (:then_4
      (CallFunction|RandomItem (Variables|Default|GetCube3)))
    (:then_5
      (CallFunction|RandomItem (Variables|Default|GetCube4)))
    (:then_6
      (CallFunction|RandomItem (Variables|Default|GetCube7)))
    (:then_7
      (CallFunction|RandomItem (Variables|Default|GetCube8)))))

(fn ConstructionScript)

(fn RandomItem
  (params (ターゲット :type Scene%20Component%20Object%20Reference))
  (bind _returnvalue (Math|Random|RandomInteger 5))
  (if (< _returnvalue 4)
    (Game|SpawnActorfromClass (Utilities|Select :Index _returnvalue :Option%200 "/Game/item/BP/Rune_Box_Kano.Rune_Box_Kano_C" :Option%201 "/Game/item/BP/Rune_Kano.Rune_Kano_C" :Option%202 "/Game/item/BP/Rune_ing.Rune_ing_C" :Option%203 "/Game/item/BP/Rune_Isa.Rune_Isa_C" :Option%204 0) (Math|Transform|MakeTransform (Transformation|GetWorldLocation ターゲット) "0, 0, 0" "0.400000,0.400000,0.400000") "Undefined" 0 0))
  (Components|DestroyComponent ターゲット))