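; Clear-check trigger actor that creates the GoalUBP widget when players reach its Box volume.
; Begin overlap counts actors tagged Player; with two or more FirstPersonCharacters in the level it waits for a count of two, otherwise it shows the widget immediately.
; The two-player branch creates the widget without adding it to the viewport.
; End overlap decrements the count, but checks the tag on the Box component, not the leaving actor.
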(event OnComponentBeginOverlap(Box)
  (params (OverlappedComponent :type Primitive%20Component%20Object%20Reference) (OtherActor :type Actor%20Object%20Reference) (OtherComp :type Primitive%20Component%20Object%20Reference) (OtherBodyIndex :type Integer) (bFromSweep :type Boolean) (SweepResult :type Hit%20Result%20Structure%20%28by%20ref%29))
  (if (Actor|ActorHasTag OtherActor "Player")
    (bind _result (Math|Integer|IncrementInt (Variables|Default|GetPlayerNum))
      (:%20%20
        (bind _outactors (Actor|GetAllActorsOfClass "/Game/FirstPersonBP/Blueprints/FirstPersonCharacter.FirstPersonCharacter_C"))
        (if (>= (Utilities|Array|Length _outactors) 2)
          (if (== _result 2)
            (UserInterface|CreateWidget "/Game/GoalUBP.GoalUBP_C"))
          (else
            (bind _returnvalue (UserInterface|CreateWidget "/Game/GoalUBP.GoalUBP_C"))
            (UserInterface|Viewport|AddtoViewport _returnvalue 0)))))))

(event OnComponentEndOverlap(Box)
  (params (OverlappedComponent :type Primitive%20Component%20Object%20Reference) (OtherActor :type Actor%20Object%20Reference) (OtherComp :type Primitive%20Component%20Object%20Reference) (OtherBodyIndex :type Integer))
  (if (Components|ComponentHasTag OverlappedComponent "Player")
    (Math|Integer|DecrementInt (Variables|Default|GetPlayerNum))))

(event EventBeginPlay)

(event Collision|EventActorBeginOverlap
  (params (OtherActor :type Actor%20Object%20Reference)))

(event EventTick
  (params (DeltaSeconds :type Float%20%28single-precision%29)))

(fn ConstructionScript)