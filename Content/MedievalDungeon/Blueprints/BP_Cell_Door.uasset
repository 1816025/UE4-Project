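; BP_Cell_Door is an unfinished cell door actor with a MoveDoor event meant to toggle it open and closed.
; It caches the first-person character at BeginPlay and derives a 90-scaled value from the camera's forward X, apparently for swing direction.
; The forward and reverse timelines, their updates and the state flag writes are disabled, and the MoveDoor function is empty.
; The door therefore never moves; the event only prints its roll when the flag is true.
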(event EventBeginPlay
  (Variables|Default|SetNewVar_0 (.AsFirst%20Person%20Character (Utilities|Casting|CastToFirstPersonCharacter (Game|GetPlayerCharacter 0)))))

(event Collision|EventActorBeginOverlap
  (params (OtherActor :type Actor%20Object%20Reference)))

(event EventTick
  (params (DeltaSeconds :type Float%20%28single-precision%29)))

(event EventMoveDoor
  (bind _returnvalue (Transformation|GetWorldRotation))
  (Variables|Default|SetPlayer%20Forward (* (.x (Math|Vector|GetForwardVector (Variables|/Game/FirstPersonBP/Blueprints/FirstPersonCharacter.FirstPersonCharacter_C|GetFirstPersonCamera (Variables|Default|GetNewVar_0)))) 9e+01))
  (if (Variables|Default|GetNewVar_1)
    (Development|PrintString (Utilities|String|ToString(Float) (.roll _returnvalue)))
    (bind _新規track_2 (Timeline|タイムライン_1 ReverseFromEnd)
      (:Update
        (CallFunction|MoveDoor (.z _新規track_2) (.roll _returnvalue))
        (Variables|Default|SetNewVar_1 false)))
    (else
      (bind _新規track_2_2 (Timeline|タイムライン_0 PlayFromStart)
        (:Update
          (CallFunction|MoveDoor (.z _新規track_2_2) (Variables|Default|GetPlayer%20Forward))
          (Variables|Default|SetNewVar_1 true))))))

(fn ConstructionScript)

(fn MoveDoor
  (params (A :type Float%20%28single-precision%29) (NewParam :type Float%20%28single-precision%29)))